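; Player knife weapon that damages overlapped actors and changes between mesh states by spending the player's blood.
; A toggleable blood mode shows the BloodBlade, enables its higher-damage overlap and activates a particle effect.
; SwitchWeapon cycles states on -1 or jumps to a given index, changing only when the MCv2 player's UseBlood succeeds.
; Cycling charges the current state's cost except on wrap to the first, while direct switching charges the target's.
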(event OnComponentBeginOverlap(knifeMesh)
  (params (OverlappedComponent :type Primitive%20Component%20Object%20Reference) (OtherActor :type Actor%20Object%20Reference) (OtherComp :type Primitive%20Component%20Object%20Reference) (OtherBodyIndex :type Integer) (bFromSweep :type Boolean) (SweepResult :type Hit%20Result%20Structure%20%28by%20ref%29))
  (Game|Damage|ApplyDamage OtherActor 1e+01 0 0))

(event OnComponentBeginOverlap(bloodBlade)
  (params (OverlappedComponent :type Primitive%20Component%20Object%20Reference) (OtherActor :type Actor%20Object%20Reference) (OtherComp :type Primitive%20Component%20Object%20Reference) (OtherBodyIndex :type Integer) (bFromSweep :type Boolean) (SweepResult :type Hit%20Result%20Structure%20%28by%20ref%29))
  (Game|Damage|ApplyDamage OtherActor 4e+01 0 0))

(event Custom|Switch%20Weapon
  (params (Weapon :type Integer))
  (if (== Weapon -1)
    ;[1 1 1] Incremental Switching
    (if (> (+ (Variables|Default|GetcurrentState) 1) 2)
      (bind _success (Default|UseBlood (Variables|Default|GetPlayer) (Utilities|Array|Get(acopy) (Variables|Default|GetstateCosts))))
      (if _success
        (bind _result (Math|Integer|IncrementInt (Variables|Default|GetcurrentState) :!label _label)
          (:%20%20
            (if (> _result 2)
              (Variables|Default|SetcurrentState 0))
            (Components|StaticMesh|SetStaticMesh (Variables|Default|GetknifeMesh) (Utilities|Array|Get(acopy) (Variables|Default|GetweaponStates) (Variables|Default|GetcurrentState))))))
      (else
        (bind _success_2 (Default|UseBlood (Variables|Default|GetPlayer) (Utilities|Array|Get(acopy) (Variables|Default|GetstateCosts) (Variables|Default|GetcurrentState))))
        (if _success_2
          (goto _label))))
    (else
      ;[1 1 1] Direct Switching
      (if (!= Weapon (Variables|Default|GetcurrentState))
        (bind _success_3 (Default|UseBlood (Variables|Default|GetPlayer) (Utilities|Array|Get(acopy) (Variables|Default|GetstateCosts) Weapon)))
        (if _success_3
          (Variables|Default|SetcurrentState Weapon)
          (Components|StaticMesh|SetStaticMesh (Variables|Default|GetknifeMesh) (Utilities|Array|Get(acopy) (Variables|Default|GetweaponStates) (Variables|Default|GetcurrentState))))))))

(event Custom|BloodOff
  (bind _bloodblade (Variables|Default|GetbloodBlade))
  ;[1 1 1] BloodGlow
  (Rendering|SetVisibility _bloodblade false false)
  (bind _output_get (Variables|/Script/Engine.PrimitiveComponent|SetbGenerateOverlapEvents _bloodblade false))
  (Variables|Default|SetbloodMode _output_get)
  (Components|Activation|Deactivate (Variables|Default|GetParticleSystem)))

(event Custom|BloodToggle
  ;[1 1 1] BloodGlow
  (if (Variables|Default|GetbloodMode)
    (CallFunction|BloodOff)
    (else
      (CallFunction|Bloodon))))

(event Custom|BloodOn
  (bind _bloodblade (Variables|Default|GetbloodBlade))
  ;[1 1 1] BloodGlow
  (Rendering|SetVisibility _bloodblade true false)
  (bind _output_get (Variables|/Script/Engine.PrimitiveComponent|SetbGenerateOverlapEvents _bloodblade true))
  (Variables|Default|SetbloodMode _output_get)
  (Components|Activation|Activate (Variables|Default|GetParticleSystem) false))

(event EventBeginPlay
  (bind _asmcv_2 (Utilities|Casting|CastToMCv2 (Game|GetPlayerCharacter 0)))
  (Variables|Default|SetPlayer _asmcv_2))

(fn ConstructionScript)