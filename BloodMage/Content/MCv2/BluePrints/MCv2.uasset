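; Player character with camera-relative movement, melee combat and a blood resource that powers weapon and ranged abilities.
; Attacks chain slash, stab and hack montages through AttackState, advancing on blend-out, locking movement and toggling knife overlap events.
; BloodMeter refills by bloodletting HitPoints or through AddBlood, drains while blood blade is active, and pays for blood bullets.
; Blade toggling and weapon switching are delegated to the bpWeapon child actor.
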(event Custom|slashONE
  (Variables|Default|SetcanMove false)
  (Animation|Montage|PlayMontage (Variables|Character|GetMesh) "/Game/MCv2/Imports/Anims/Montages/horiSlash.horiSlash"
    (:then
      (Variables|Default|SetattackState 3))
    (:OnCompleted
      (Variables|Default|SetcanMove true)
      (Variables|Default|SetattackState 0)
      (Variables|/Script/Engine.PrimitiveComponent|SetbGenerateOverlapEvents (Variables|/Game/MCv2/Knife/BluePrints/bpWeapon.bpWeapon_C|GetknifeMesh (.AsBp%20Weapon (Utilities|Casting|CastTobpWeapon (Variables|/Script/Engine.ChildActorComponent|GetChildActor (Variables|Default|GetWeapon))))) false))
    (:OnBlendOut
      (Variables|Default|SetattackState 1))))

(event Custom|stabTWO
  (Variables|Default|SetcanMove false)
  (Animation|Montage|PlayMontage (Variables|Character|GetMesh) "/Game/MCv2/Imports/Anims/Montages/Stab.Stab"
    (:then
      (Variables|Default|SetattackState 3))
    (:OnCompleted
      (Variables|Default|SetcanMove true)
      (Variables|Default|SetattackState 0)
      (Variables|/Script/Engine.PrimitiveComponent|SetbGenerateOverlapEvents (Variables|/Game/MCv2/Knife/BluePrints/bpWeapon.bpWeapon_C|GetknifeMesh (.AsBp%20Weapon (Utilities|Casting|CastTobpWeapon (Variables|/Script/Engine.ChildActorComponent|GetChildActor (Variables|Default|GetWeapon))))) false))
    (:OnBlendOut
      (Variables|Default|SetattackState 2))))

(event Custom|hackTHREE
  (Variables|Default|SetcanMove false)
  (Animation|Montage|PlayMontage (Variables|Character|GetMesh) "/Game/MCv2/Imports/Anims/Montages/vertSlash.vertSlash"
    (:then
      (Variables|Default|SetattackState 3))
    (:OnCompleted
      (Variables|Default|SetcanMove true)
      (Variables|Default|SetattackState 0)
      (Variables|/Script/Engine.PrimitiveComponent|SetbGenerateOverlapEvents (Variables|/Game/MCv2/Knife/BluePrints/bpWeapon.bpWeapon_C|GetknifeMesh (.AsBp%20Weapon (Utilities|Casting|CastTobpWeapon (Variables|/Script/Engine.ChildActorComponent|GetChildActor (Variables|Default|GetWeapon))))) false))))

(event Custom|tryAttack
  (Variables|/Script/Engine.PrimitiveComponent|SetbGenerateOverlapEvents (Variables|/Game/MCv2/Knife/BluePrints/bpWeapon.bpWeapon_C|GetknifeMesh (.AsBp%20Weapon (Utilities|Casting|CastTobpWeapon (Variables|/Script/Engine.ChildActorComponent|GetChildActor (Variables|Default|GetWeapon))))) true)
  (switch int (Variables|Default|GetattackState)
    (:0
      (CallFunction|SlashONE))
    (:1
      (CallFunction|StabTWO))
    (:2
      (CallFunction|HackTHREE))))

(event EventBeginPlay)

(event Collision|EventActorBeginOverlap
  (params (OtherActor :type Actor%20Object%20Reference)))

(event EventTick
  (params (DeltaSeconds :type Float%20%28single-precision%29))
  (bind _asbp_weapon (Utilities|Casting|CastTobpWeapon (Variables|/Script/Engine.ChildActorComponent|GetChildActor (Variables|Default|GetWeapon))))
  (if (Variables|/Game/MCv2/Knife/BluePrints/bpWeapon.bpWeapon_C|GetbloodMode _asbp_weapon)
    (bind _output_get (Variables|Default|SetbloodMeter (Math|Float|Clamp(Float) (- (Variables|Default|GetbloodMeter) (* DeltaSeconds 5.0)) 0.0 (Variables|Default|GetMaxBlood))))
    (if (<= _output_get 0.0)
      (Default|BloodOff _asbp_weapon))))

(event Input|ActionEvents|InputActionAttack
  (params (Key :type Key%20Structure))
  (:Pressed
    (Variables|Default|SetinCombat true)
    (CallFunction|TryAttack)
    (Utilities|FlowControl|RetriggerableDelay 3.0)
    (Variables|Default|SetinCombat false)))

(event Input|ActionEvents|InputActionSwitchBloodWeapon
  (params (Key :type Key%20Structure))
  ;[1 1 1] Weapon Switching
  (:Pressed
    (bind _asbp_weapon (Utilities|Casting|CastTobpWeapon (Variables|/Script/Engine.ChildActorComponent|GetChildActor (Variables|Default|GetWeapon))))
    (if (== Key "LeftShift")
      (Default|SwitchWeapon _asbp_weapon -1)
      (elif (== Key "One")
        (Default|SwitchWeapon _asbp_weapon 0)
        (elif (== Key "Two")
          (Default|SwitchWeapon _asbp_weapon 1)
          (else
            (Default|SwitchWeapon _asbp_weapon 2)))))))

(event Input|ActionEvents|InputActiontoggleBloodBlade
  (params (Key :type Key%20Structure))
  (:Pressed
    (if (> (Variables|Default|GetbloodMeter) 0.0)
      (bind _asbp_weapon (Utilities|Casting|CastTobpWeapon (Variables|/Script/Engine.ChildActorComponent|GetChildActor (Variables|Default|GetWeapon))))
      (Default|BloodToggle _asbp_weapon))))

(event Input|ActionEvents|InputActionShootProjectile
  (params (Key :type Key%20Structure))
  ;[1 1 1] Shoot Blood Bullet
  (:Pressed
    (bind _success (CallFunction|UseBlood 5.0))
    (if _success
      (Game|SpawnActorfromClass "/Game/MCv2/BloodBullet.BloodBullet_C" (Transformation|GetActorTransform) "Undefined" 0 self))))

(event Input|AxisEvents|InputAxisMoveX
  (params (AxisValue :type Float%20%28single-precision%29))
  ;[1 1 1] Movement
  (if (Variables|Default|GetcanMove)
    (Pawn|Input|AddMovementInput (Math|Vector|GetRightVector (Math|Rotator|MakeRotator 0.0 0.0 (.yaw (Pawn|GetControlRotation :!class /Script/Engine.Pawn)))) AxisValue false)))

(event Input|AxisEvents|InputAxisMoveY
  (params (AxisValue :type Float%20%28single-precision%29))
  ;[1 1 1] Movement
  (if (Variables|Default|GetcanMove)
    (Pawn|Input|AddMovementInput (Math|Vector|GetForwardVector (Math|Rotator|MakeRotator 0.0 0.0 (.yaw (Pawn|GetControlRotation :!class /Script/Engine.Pawn)))) AxisValue false)))

(event Input|AxisEvents|InputAxisCameraPitch
  (params (AxisValue :type Float%20%28single-precision%29))
  ;[1 1 1] Camera
  (Class|PlayerController|AddPitchInput (Game|GetPlayerController 0) (* AxisValue (Utilities|Time|GetWorldDeltaSeconds) 9e+01)))

(event Input|AxisEvents|InputAxisCameraYaw
  (params (AxisValue :type Float%20%28single-precision%29))
  ;[1 1 1] Camera
  (Class|PlayerController|AddYawInput (Game|GetPlayerController 0) (* AxisValue (Utilities|Time|GetWorldDeltaSeconds) 1.8e+02)))

(event Input|AxisEvents|InputAxisBloodLetting
  (params (AxisValue :type Float%20%28single-precision%29))
  ;[1 1 1] BloodLetting
  (if (and (< (Variables|Default|GetbloodMeter) (Variables|Default|GetMaxBlood)) (> (Variables|Default|GetHitPoints) 2.0))
    (Variables|Default|SetHitPoints (- (Variables|Default|GetHitPoints) AxisValue))
    (Variables|Default|SetbloodMeter (+ (Variables|Default|GetbloodMeter) AxisValue))))

(fn ConstructionScript)

(fn AddBlood
  (params (Blood :type Float%20%28single-precision%29))
  (bind _output_get (Variables|Default|SetbloodMeter (Math|Float|Clamp(Float) (+ (Variables|Default|GetbloodMeter) Blood) 0.0 (Variables|Default|GetMaxBlood))))
  (return _output_get))

(fn UseBlood
  (params (Cost :type Float%20%28single-precision%29))
  (bind _available (CallFunction|CheckBlood Cost))
  (if _available
    (Variables|Default|SetbloodMeter (Math|Float|Clamp(Float) (- (Variables|Default|GetbloodMeter) Cost) 0.0 (Variables|Default|GetMaxBlood))))
  (return (Variables|Default|GetbloodMeter) _available))

(fn CheckBlood
  (params (Cost :type Float%20%28single-precision%29))
  (return (>= (Variables|Default|GetbloodMeter) Cost)))