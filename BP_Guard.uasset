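; Guard AI pawn that patrols a chain of waypoints and chases the player on sight.
; Tick switches on CurrentState, issuing AI MoveTo toward either the patrol waypoint, which hands on its next node after a pause, or the player.
; FarSenses triggers the chase; reaching the player prints a caught message and restores patrol.
; CloseSenses is an empty stub, and AlertUp, a debug-printed alert counter, is uncalled here.
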(event OnSeePawn(FarSenses)
  (params (Pawn :type Pawn%20Object%20Reference))
  (if (== Pawn (Variables|Default|GetPlayer))
    (Variables|Default|SetClose true)
    (Variables|Default|SetCurrentState 1)
    (Utilities|FlowControl|Delay 0.2)
    (Variables|Default|SetPawnSeen 0)))

(event OnSeePawn(CloseSenses)
  (params (Pawn :type Pawn%20Object%20Reference)))

(event EventBeginPlay)

(event Collision|EventActorBeginOverlap
  (params (OtherActor :type Actor%20Object%20Reference)))

(event EventTick
  (params (DeltaSeconds :type Float%20%28single-precision%29))
  (switch int (Variables|Default|GetCurrentState)
    (:0
      (AI|AIMoveTo self "0, 0, 0" (Variables|Default|GetPatrolWaypoint) 2.0 false
        (:OnSuccess
          (bind _aswaypoint (Utilities|Casting|CastToWaypoint (Variables|Default|GetPatrolWaypoint)))
          (bind _nextwaypoint (Default|NextWaypointNode _aswaypoint))
          (Utilities|FlowControl|Delay 4.0)
          (CallFunction|ContintuetoPatrol _nextwaypoint))))
    (:1
      (AI|AIMoveTo self "0, 0, 0" (Variables|Default|GetPlayer) 1e+02 false
        (:OnSuccess
          (Variables|Default|SetCurrentState 0)
          (Development|PrintString "I caught you" true true "(R=0.000000,G=0.660000,B=1.000000,A=1.000000)" 1e+01)
          (Utilities|FlowControl|Delay 1e+01))))))

(fn ConstructionScript)

(fn ContintuetoPatrol
  (params (NewWaypoint :type Waypoint%20Object%20Reference))
  (Variables|Default|SetPatrolWaypoint NewWaypoint))

(fn AlertUp
  (bind _result (Math|Integer|IncrementInt (Variables|Default|GetAlertLevel))
    (:%20%20
      (Development|PrintString "Enter Alert Level" true false "(R=0.000000,G=0.660000,B=1.000000,A=1.000000)" 1e+01)
      (Development|PrintString (Utilities|String|ToString(Integer) _result) true true "(R=0.000000,G=0.660000,B=1.000000,A=1.000000)" 1e+01))))